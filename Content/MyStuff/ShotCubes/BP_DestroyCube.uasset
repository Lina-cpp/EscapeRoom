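; BP_DestroyCube is a shootable target cube that scores a point for the player in the escape room game.
; On BeginPlay it casts the game mode to BP_EscapeRoomGameMode and caches the reference.
; When its static mesh is hit by a BP_FirstPersonProjectile, it destroys itself, increments the game mode's Points and prints the new total.
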(event `self.ReceiveActorBeginOverlap`
  (params (OtherActor :type "Actor Object Reference")))

(event `self.ReceiveBeginPlay`
  ;[1 1 1] Cast to BP_Gamemode and make it Variable
  (bind _asbp_escape_room_game_mode (cast `/Game/MyStuff/BP_EscapeRoomGameMode` (`GameplayStatics.GetGameMode`)))
  (set `self.As BP Escape Room Game Mode` _asbp_escape_room_game_mode))

(event `self.StaticMeshComponent.OnComponentHit`
  (params (HitComponent :type "PrimitiveComponent Object Reference") (OtherActor :type "Actor Object Reference") (OtherComp :type "PrimitiveComponent Object Reference") (NormalImpulse :type "Vector Structure") (Hit :type "HitResult Structure (by ref)"))
  (bind _as_bp_escape_room_game_mode (`self.As BP Escape Room Game Mode`))
  ;[1 1 1] OnHit - Destroy Cube and add point
  (cast `/Game/FirstPerson/Blueprints/BP_FirstPersonProjectile` OtherActor)
  (`self.K2_DestroyActor`)
  (bind _output_get (set `/Game/MyStuff/BP_EscapeRoomGameMode.Points` (+ 1 (`/Game/MyStuff/BP_EscapeRoomGameMode.Points` _as_bp_escape_room_game_mode)) _as_bp_escape_room_game_mode))
  (`KismetSystemLibrary.PrintString` (`KismetStringLibrary.Conv_IntToString` _output_get)))

(fn `UserConstructionScript`)