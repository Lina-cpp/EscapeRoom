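; BP_MySaves stores a scoreboard of minute, second and millisecond times, apparently for saving, exposed through GetScores.
; AddTime appends a time and bubbles it up in a backward pass, ordering longest first via CompareTimes, which adds unscaled milliseconds to total seconds.
; The repeat flag is only ever set false here, and the over-ten trim loops from length to 9, so it removes nothing.
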(fn `AddTime`
  (params (Struct :type "/Game/MyStuff/SavingGame/ST_SaveGame1 Structure"))
  (locals (HasChangesScoreboard :type Boolean))
  (bind _struct (`self.Struct`))
  (bind _struct_2 (`self.Struct`))
  (bind _returnvalue (`KismetArrayLibrary.Array_Add` _struct Struct))
  (if (!= _returnvalue 0)
    (bind _arrayindex (`/Engine/EditorBlueprintResources/StandardMacros.ReverseForEachLoop` _struct :!label _label)
      (:`LoopBody`
        (if (> _arrayindex 0)
          (bind _returnvalue_2 (- _arrayindex 1))
          (bind _istime2bigger (`self.Compare Times` (`|GetArrayItem` _struct_2 _returnvalue_2) (`|GetArrayItem` _struct_2 _arrayindex)))
          (if (not _istime2bigger)
            (`KismetArrayLibrary.Array_Swap` _struct_2 _returnvalue_2 _arrayindex)
            (set `local.HasChangesScoreboard` false))))
      (:`Completed`
        (if (`local.HasChangesScoreboard`)
          (set `local.HasChangesScoreboard` false)
          (goto _label)
          (elif (> (`KismetArrayLibrary.Array_Length` (`self.Struct`)) 10)
            (for _index (range (`KismetArrayLibrary.Array_Length` (`self.Struct`)) 10)
              (`KismetArrayLibrary.Array_Remove` (`self.Struct`) _index))))))))

(fn `Compare Times`
  (params (`Time 1` :type "/Game/MyStuff/SavingGame/ST_SaveGame1 Structure") (`Time 2` :type "/Game/MyStuff/SavingGame/ST_SaveGame1 Structure"))
  (returns (IsTime2Bigger :type Boolean))
  (bind (_miliseconds _seconds _minutes) (break `/Game/MyStuff/SavingGame/ST_SaveGame1` `Time 1`))
  (bind (_miliseconds_2 _seconds_2 _minutes_2) (break `/Game/MyStuff/SavingGame/ST_SaveGame1` `Time 2`))
  (if (> (+ _miliseconds (+ _seconds (* _minutes 60))) (+ _miliseconds_2 (+ _seconds_2 (* _minutes_2 60))))
    (return true)
    (else
      (return false))))

(fn `Get Scores`
  (returns (Scores :type "Array of /Game/MyStuff/SavingGame/ST_SaveGame1 Structure"))
  (return (`self.Struct`)))