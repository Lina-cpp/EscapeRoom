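; BP_Cell_Door is a dungeon cell door that swings open when the player enters its trigger box and closes when they leave.
; On overlap, a dot product of the player's and door's forward vectors picks one of two swing angles based on the player's facing.
; A timeline scales that angle into the door mesh's relative yaw, playing on entry and reversing on exit.
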(event `self.Box.OnComponentBeginOverlap`
  (params (OverlappedComponent :type "PrimitiveComponent Object Reference") (OtherActor :type "Actor Object Reference") (OtherComp :type "PrimitiveComponent Object Reference") (OtherBodyIndex :type Integer) (bFromSweep :type Boolean) (SweepResult :type "HitResult Structure (by ref)"))
  (bind _sm_cell_door (`self.SM_Cell_Door`))
  (bind _asbp_player (cast `/Game/BP_Player` OtherActor))
  (set `self.PlayerFacingDoors` (>= (`KismetMathLibrary.Dot_VectorVector` (`self.GetActorForwardVector` _asbp_player) (`SceneComponent.GetForwardVector` (`self.DefaultSceneRoot`))) 0.0))
  (bind (_direction _newtrack_0) (`Timeline|Timeline_Door` :!label _label)
    (:`Update`
      (if (`self.PlayerFacingDoors`)
        (`SceneComponent.K2_SetRelativeRotation` _sm_cell_door (`KismetMathLibrary.MakeRotator` 0.0 0.0 (* _newtrack_0 (`self.angle 1`))) false false)
        (else
          (`SceneComponent.K2_SetRelativeRotation` _sm_cell_door (`KismetMathLibrary.MakeRotator` 0.0 0.0 (* _newtrack_0 (`self.angle 2`))) false false))))))

(event `self.Box.OnComponentEndOverlap`
  (params (OverlappedComponent :type "PrimitiveComponent Object Reference") (OtherActor :type "Actor Object Reference") (OtherComp :type "PrimitiveComponent Object Reference") (OtherBodyIndex :type Integer))
  (cast `/Game/BP_Player` OtherActor)
  (goto _label :!via `Reverse`))

(fn `UserConstructionScript`)